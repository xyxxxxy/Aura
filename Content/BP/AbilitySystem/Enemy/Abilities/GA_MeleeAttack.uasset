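; Enemy melee attack gameplay ability that turns the avatar toward its combat target and plays a random attack montage.
; Avatar data such as target, montages and socket location comes through message calls.
; A gameplay event matching a montage tag triggers a radius query at the combat socket, damaging live non-friendly players, then ends the ability.
; It also ends when no montages exist or the montage completes, is interrupted or is cancelled.
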(event `self.K2_ActivateAbility`
  (bind _returnvalue (`self.GetAvatarActorFromActorInfo`))
  (bind _returnvalue_2 (`self.GetAvatarActorFromActorInfo`))
  (bind _returnvalue_3 (message `EnemyInterface.GetCombatTarget` _returnvalue_2))
  (message `CombatInterface.UpdateFacingTarget` _returnvalue_2 (`Actor.K2_GetActorLocation` _returnvalue_3))
  (bind _returnvalue_4 (message `CombatInterface.GetAttackMontages` _returnvalue_2))
  (if (`KismetArrayLibrary.Array_IsEmpty` _returnvalue_4)
    (`self.K2_EndAbility`)
    (else
      (bind _outitem (`KismetArrayLibrary.Array_Random` _returnvalue_4))
      (`AbilityTask_PlayMontageAndWait.CreatePlayMontageAndWaitProxy` "None" (break `TaggedMontage` _outitem)
        (:`then`
          (`AbilityTask_WaitGameplayEvent.WaitGameplayEvent` (`.MontageTag` (break `TaggedMontage` _outitem)) null
            (:`EventReceived`
              (bind _returnvalue_5 (message `CombatInterface.GetCombatSocketLocation` _returnvalue (`.MontageTag` (break `TaggedMontage` _outitem))))
              (bind _outoverlappingactors (`AuraAbilitySystemLibrary.GetLivePlayersWithRadius` _returnvalue (`|MakeArray` _returnvalue) 100.0 _returnvalue_5))
              (for _array_element _outoverlappingactors
                (if (`AuraAbilitySystemLibrary.IsNotFriend` (`self.GetAvatarActorFromActorInfo`) _array_element)
                  (`self.CauseDamage` _array_element)))
              (`self.K2_EndAbility`))))
        (:`OnCompleted`
          (`self.K2_EndAbility` :!label _label))
        (:`OnInterrupted`
          (goto _label))
        (:`OnCancelled`
          (goto _label))))))