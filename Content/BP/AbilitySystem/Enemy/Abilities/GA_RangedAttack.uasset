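; Enemy ranged attack gameplay ability that turns the avatar toward its combat target and fires a projectile at it.
; It plays a random attack montage from the avatar, or ends immediately if none exist.
; A gameplay event, tagged from a separately evaluated Random pick, triggers SpawnProjectile at the target's current location.
; The ability ends when the montage completes, is interrupted or is cancelled.
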(event `self.K2_ActivateAbility`
  (bind _returnvalue (`self.GetAvatarActorFromActorInfo`))
  (bind _returnvalue_2 (message `EnemyInterface.GetCombatTarget` _returnvalue))
  (message `CombatInterface.UpdateFacingTarget` _returnvalue (`Actor.K2_GetActorLocation` _returnvalue_2))
  (bind _returnvalue_3 (message `CombatInterface.GetAttackMontages` _returnvalue))
  (if (`KismetArrayLibrary.Array_IsEmpty` _returnvalue_3)
    (`self.K2_EndAbility`)
    (else
      (bind _outitem (`KismetArrayLibrary.Array_Random` _returnvalue_3))
      (`AbilityTask_PlayMontageAndWait.CreatePlayMontageAndWaitProxy` "None" (break `TaggedMontage` _outitem) 1.0 "None" false
        (:`then`
          (`AbilityTask_WaitGameplayEvent.WaitGameplayEvent` (`.MontageTag` (break `TaggedMontage` _outitem)) null
            (:`EventReceived`
              (bind _returnvalue_4 (message `EnemyInterface.GetCombatTarget` (`self.GetAvatarActorFromActorInfo`)))
              (`self.SpawnProjectile` (`Actor.K2_GetActorLocation` _returnvalue_4)))))
        (:`OnCompleted`
          (`self.K2_EndAbility` :!label _label))
        (:`OnInterrupted`
          (goto _label))
        (:`OnCancelled`
          (goto _label))))))